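; Base weapon Blueprint that starts auto-firing on BeginPlay and signals each shot through a Shooted call, leaving projectile spawning out of this graph.
; A looping timer at 1/FireRate paces shots, and fire rate changes wait out the remaining cooldown before restarting or stopping.
; Barrels are runtime-added arrow components centred along local Y by count and spacing.
; ChangeStat sets projectile damage or fire rate by stat category.
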(event `self.ReceiveBeginPlay`
  (`self.StartShooting`))

(event `SetShootAvailable`
  (set `self.IsShootAvailable` true)
  (if (`self.IsShooting`)
    (`self.Shoot` false)
    (else
      (`KismetSystemLibrary.K2_ClearAndInvalidateTimerHandle` (`self.ShootTimer`)))))

(event `Shoot`
  (params (AffectedBySkill :type Boolean))
  (`self.Shooted` AffectedBySkill)
  (set `self.IsShootAvailable` false))

(event `FireRateChanged`
  (set `self.Wait` (`KismetSystemLibrary.K2_GetTimerRemainingTimeHandle` (`self.ShootTimer`)))
  (`KismetSystemLibrary.K2_ClearAndInvalidateTimerHandle` (`self.ShootTimer`))
  (`KismetSystemLibrary.Delay` (`self.Wait`))
  (if (!= (`self.FireRate`) 0.0)
    (`self.SetShootAvailable`)
    (`self.StartShooting`)
    (else
      (`self.StopShooting`)
      (`self.SetShootAvailable`))))

(event `/Game/Blueprints/InventoryEquipment/Interface/BPI_ItemInterface.ChangeStat`
  (params (StatCategory :type "/Game/Blueprints/InventoryEquipment/Enum/E_StatCategory Enum" :default "NewEnumerator0") (StatAmount :type "Float (single-precision)"))
  (switch `/Game/Blueprints/InventoryEquipment/Enum/E_StatCategory` StatCategory
    (:`NewEnumerator0`
      (set `self.ProjectileDamage` StatAmount))
    (:`NewEnumerator3`
      (`self.SetFireRate` StatAmount))))

(fn `AddBarrelCount`
  (params (Delta :type "Float (double-precision)"))
  (bind _output_get (set `self.BarrelCount` (+ (`self.BarrelCount`) Delta)))
  (`KismetArrayLibrary.Array_Clear` (`self.Barrels`))
  (bind _returnvalue (- _output_get 1.0))
  (for _index (range (+ (`KismetMathLibrary.FTrunc` _returnvalue) 1))
    (bind _returnvalue_2 (`AddComponent|NODE_AddArrowComponent-1` :`RelativeTransform` (`KismetMathLibrary.MakeTransform` (`KismetMathLibrary.MakeVector` 0.0 (- (* _index (`self.BarrelDistance`)) (/ (* _returnvalue (`self.BarrelDistance`)) 2.0))))))
    (`KismetArrayLibrary.Array_Add` (`self.Barrels`) _returnvalue_2)))

(fn `AddBarrelDistance`
  (params (Delta :type "Float (double-precision)"))
  (set `self.BarrelDistance` (+ (`self.BarrelDistance`) Delta))
  (for (_array_element _array_index) (`self.Barrels`)
    (`SceneComponent.K2_SetRelativeLocation` _array_element (`KismetMathLibrary.MakeVector` 0.0 (- (* _array_index (`self.BarrelDistance`)) (/ (* (- (`self.BarrelCount`) 1.0) (`self.BarrelDistance`)) 2.0))) false false)))

(fn `AddFireRate`
  (params (Delta :type "Float (double-precision)"))
  (set `self.FireRate` (+ (`self.FireRate`) Delta))
  (`self.FireRateChanged`))

(fn `SetBarrelCount`
  (params (Value :type "Float (double-precision)"))
  (bind _output_get (set `self.BarrelCount` Value))
  (`KismetArrayLibrary.Array_Clear` (`self.Barrels`))
  (bind _returnvalue (- _output_get 1.0))
  (for _index (range (+ (`KismetMathLibrary.FTrunc` _returnvalue) 1))
    (bind _returnvalue_2 (`AddComponent|NODE_AddArrowComponent-2` :`RelativeTransform` (`KismetMathLibrary.MakeTransform` (`KismetMathLibrary.MakeVector` 0.0 (- (* _index (`self.BarrelDistance`)) (/ (* _returnvalue (`self.BarrelDistance`)) 2.0))))))
    (`KismetArrayLibrary.Array_Add` (`self.Barrels`) _returnvalue_2)))

(fn `SetBarrelDistance`
  (params (Value :type "Float (double-precision)"))
  (set `self.BarrelDistance` Value)
  (for (_array_element _array_index) (`self.Barrels`)
    (`SceneComponent.K2_SetRelativeLocation` _array_element (`KismetMathLibrary.MakeVector` 0.0 (- (* _array_index (`self.BarrelDistance`)) (/ (* (- (`self.BarrelCount`) 1.0) (`self.BarrelDistance`)) 2.0))) false false)))

(fn `SetFireRate`
  (params (Value :type "Float (double-precision)"))
  (set `self.FireRate` Value)
  (`self.FireRateChanged`))

(fn `StartShooting`
  (set `self.IsShooting` true)
  (if (`self.IsShootAvailable`)
    (`self.Shoot` false))
  (bind _returnvalue (`KismetSystemLibrary.K2_SetTimerDelegate` (`|CreateDelegate` :!event `SetShootAvailable`) (/ 1.0 (`self.FireRate`)) true))
  (set `self.ShootTimer` _returnvalue))

(fn `StopShooting`
  (set `self.IsShooting` false))

(fn `UserConstructionScript`)