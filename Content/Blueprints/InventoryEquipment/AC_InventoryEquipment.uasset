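; Player controller component that manages a networked inventory and equipment system, creating its UI for the local player and granting two starter items on the server.
; Items live in maps keyed by item type, with an ID map tracking each location.
; S_ events run authoritative SER functions, then M_ events mirror successful changes on remotes through CLI functions and dispatchers.
; Equipping checks slot limits and spawns item actors attached to controller-provided sockets.
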(event `self.ReceiveBeginPlay`
  (bind _asbp_in_game_player_controller (cast `/Game/Blueprints/Player/BP_InGamePlayerController` (`self.GetOwner`)))
  (bind _output_get (set `self.InGamePlayerController` _asbp_in_game_player_controller))
  (`|ExecutionSequence`
    (:`then_0`
      (if (`Controller.IsLocalPlayerController` _output_get)
        (bind _returnvalue (`|CreateWidget` "/Game/Blueprints/InventoryEquipment/Widget/W_InventoryEquipment.W_InventoryEquipment_C" (`self.InGamePlayerController`) self))
        (`/Game/Blueprints/Player/BP_PlayerControllerBase.AddWidget` (`self.InGamePlayerController`) _returnvalue "P")))
    (:`then_1`
      (if (`Actor.HasAuthority` _output_get)
        (`KismetSystemLibrary.Delay` 2.0)
        (bind _returnvalue_2 (`|GetDataTableRow` "/Game/Blueprints/InventoryEquipment/DT_Items.DT_Items" "LF-1")
          (:`then`
            (`self.S_AddItemToInventory` _returnvalue_2)
            (bind _returnvalue_3 (`|GetDataTableRow` "/Game/Blueprints/InventoryEquipment/DT_Items.DT_Items" "SH-1")
              (:`then`
                (`self.S_AddItemToInventory` _returnvalue_3)))))))))

(event `S_AddItemToInventory`
  (params (Item :type "/Game/Blueprints/InventoryEquipment/Struct/S_Item Structure"))
  ;[1 1 1] AddItemToInventory
  (bind (_added _addeditem) (`self.SER_AddItemToInventory` Item))
  (if _added
    (`self.M_AddItemToInventory` _addeditem)))

(event `S_AddItemToEquipment`
  (params (Item :type "/Game/Blueprints/InventoryEquipment/Struct/S_Item Structure"))
  ;[1 1 1] AddItemToEquipment
  (bind (_added _addeditem) (`self.SER_AddItemToEquipment` Item))
  (if _added
    (`self.M_AddItemToEquipment` _addeditem)))

(event `M_AddItemToInventory`
  (params (Item :type "/Game/Blueprints/InventoryEquipment/Struct/S_Item Structure"))
  ;[1 1 1] AddItemToInventory
  (`self.SwitchHasAuthority`
    (:`Remote`
      (`self.CLI_AddItemToInventory` Item))))

(event `M_AddItemToEquipment`
  (params (Item :type "/Game/Blueprints/InventoryEquipment/Struct/S_Item Structure"))
  ;[1 1 1] AddItemToEquipment
  (`self.SwitchHasAuthority`
    (:`Remote`
      (`self.CLI_AddItemToEquipment` Item))))

(event `S_SendItemToInventory`
  (params (Item :type "/Game/Blueprints/InventoryEquipment/Struct/S_Item Structure"))
  ;[1 1 1] SendItemToInventory
  (bind (_sended _addeditem) (`self.SER_SendItemToInventory` Item))
  (if _sended
    (`self.M_SendItemToInventory` _addeditem)))

(event `S_SendItemToEquipment`
  (params (Item :type "/Game/Blueprints/InventoryEquipment/Struct/S_Item Structure"))
  ;[1 1 1] SendItemToEquipment
  (bind (_sended _addeditem) (`self.SER_SendItemToEquipment` Item))
  (if _sended
    (`self.M_SendItemToEquipment` _addeditem)))

(event `M_SendItemToInventory`
  (params (Item :type "/Game/Blueprints/InventoryEquipment/Struct/S_Item Structure"))
  ;[1 1 1] SendItemToInventory
  (`self.SwitchHasAuthority`
    (:`Remote`
      (`self.CLI_SendItemToInventory` Item))))

(event `M_SendItemToEquipment`
  (params (Item :type "/Game/Blueprints/InventoryEquipment/Struct/S_Item Structure"))
  ;[1 1 1] SendItemToEquipment
  (`self.SwitchHasAuthority`
    (:`Remote`
      (`self.CLI_SendItemToEquipment` Item))))

(fn `CLI_AddItemToEquipment`
  (params (Item :type "/Game/Blueprints/InventoryEquipment/Struct/S_Item Structure"))
  (returns (Added :type Boolean))
  (locals (ItemRef :type "/Game/Blueprints/InventoryEquipment/Struct/S_Item Structure") (ItemTypeRef :type "/Game/Blueprints/InventoryEquipment/Enum/E_ItemType Enum") (ItemArrayRef :type "Array of /Game/Blueprints/InventoryEquipment/Struct/S_Item Structure") (ItemAddedIndex :type Integer))
  (bind _output_get (set `local.ItemRef` Item))
  (bind _output_get_2 (set `local.ItemTypeRef` (`.ItemType_35_B85020CC4326255BF9CA7986369ED08C` (break `/Game/Blueprints/InventoryEquipment/Struct/S_Item` _output_get))))
  (bind _output_get_3 (set `local.ItemArrayRef` (`.Array_3_54825DA340DDAE3ADDAE89ABB7425895` (break `/Game/Blueprints/InventoryEquipment/Struct/S_ItemArray` (`BlueprintMapLibrary.Map_Find` (`self.EquipmentMap`) _output_get_2)))))
  (bind _returnvalue (`KismetArrayLibrary.Array_Add` _output_get_3 (`local.ItemRef`)))
  (set `local.ItemAddedIndex` _returnvalue)
  (`BlueprintMapLibrary.Map_Add` (`self.EquipmentMap`) (`local.ItemTypeRef`) (make `/Game/Blueprints/InventoryEquipment/Struct/S_ItemArray` (`local.ItemArrayRef`)))
  (`KismetArrayLibrary.Array_Clear` (`local.ItemArrayRef`))
  (`BlueprintMapLibrary.Map_Add` (`self.InventoryIDs`) (`.ID_34_480AFE364D7F3357C84857B4B302F81E` (break `/Game/Blueprints/InventoryEquipment/Struct/S_Item` (`local.ItemRef`))) (make `/Game/Blueprints/InventoryEquipment/Struct/S_ItemLocation` "NewEnumerator1" (`local.ItemTypeRef`) (`local.ItemAddedIndex`)))
  (`self.ItemAddedToEquipment` (`local.ItemRef`))
  (return true))

(fn `CLI_AddItemToInventory`
  (params (Item :type "/Game/Blueprints/InventoryEquipment/Struct/S_Item Structure"))
  (returns (Added :type Boolean))
  (locals (ItemArrayRef :type "Array of /Game/Blueprints/InventoryEquipment/Struct/S_Item Structure") (ItemTypeRef :type "/Game/Blueprints/InventoryEquipment/Enum/E_ItemType Enum") (ItemAddedIndex :type Integer :default 0))
  (bind ((`ID_34_480AFE364D7F3357C84857B4B302F81E` _id) (`ItemType_35_B85020CC4326255BF9CA7986369ED08C` _itemtype)) (break `/Game/Blueprints/InventoryEquipment/Struct/S_Item` (`local.Item`)))
  (bind _output_get (set `local.ItemTypeRef` (`.ItemType_35_B85020CC4326255BF9CA7986369ED08C` (break `/Game/Blueprints/InventoryEquipment/Struct/S_Item` Item))))
  (bind _output_get_2 (set `local.ItemArrayRef` (`.Array_3_54825DA340DDAE3ADDAE89ABB7425895` (break `/Game/Blueprints/InventoryEquipment/Struct/S_ItemArray` (`BlueprintMapLibrary.Map_Find` (`self.InventoryMap`) _output_get)))))
  (bind _returnvalue (`KismetArrayLibrary.Array_Add` _output_get_2 (`local.Item`)))
  (set `local.ItemAddedIndex` _returnvalue)
  (`BlueprintMapLibrary.Map_Add` (`self.InventoryMap`) (`.ItemType_35_B85020CC4326255BF9CA7986369ED08C` (break `/Game/Blueprints/InventoryEquipment/Struct/S_Item` (`local.Item`))) (make `/Game/Blueprints/InventoryEquipment/Struct/S_ItemArray` (`local.ItemArrayRef`)))
  (`KismetArrayLibrary.Array_Clear` (`local.ItemArrayRef`))
  (`BlueprintMapLibrary.Map_Add` (`self.InventoryIDs`) _id (make `/Game/Blueprints/InventoryEquipment/Struct/S_ItemLocation` "NewEnumerator0" _itemtype))
  (`self.ItemAddedToInventory` (`local.Item`))
  (return true))

(fn `CLI_SendItemToEquipment`
  (params (Item :type "/Game/Blueprints/InventoryEquipment/Struct/S_Item Structure"))
  (returns (Sended :type Boolean))
  (locals (ItemArrayRef :type "Array of /Game/Blueprints/InventoryEquipment/Struct/S_Item Structure") (ItemLocationRef :type "/Game/Blueprints/InventoryEquipment/Struct/S_ItemLocation Structure"))
  (bind (_itemlocation _itemtype _index) (break `/Game/Blueprints/InventoryEquipment/Struct/S_ItemLocation` (`BlueprintMapLibrary.Map_Find` (`self.InventoryIDs`) (`.ID_34_480AFE364D7F3357C84857B4B302F81E` (break `/Game/Blueprints/InventoryEquipment/Struct/S_Item` (`local.Item`))))))
  (`self.CLI_AddItemToEquipment` Item)
  (bind _output_get (set `local.ItemArrayRef` (`.Array_3_54825DA340DDAE3ADDAE89ABB7425895` (break `/Game/Blueprints/InventoryEquipment/Struct/S_ItemArray` (`BlueprintMapLibrary.Map_Find` (`self.InventoryMap`) _itemtype)))))
  (`KismetArrayLibrary.Array_Remove` _output_get _index)
  (`BlueprintMapLibrary.Map_Add` (`self.InventoryMap`) (`.ItemType_35_B85020CC4326255BF9CA7986369ED08C` (break `/Game/Blueprints/InventoryEquipment/Struct/S_Item` (`local.Item`))) (make `/Game/Blueprints/InventoryEquipment/Struct/S_ItemArray` (`local.ItemArrayRef`)))
  (`self.ItemRemovedFromInventory` (`local.Item`))
  (return true))

(fn `CLI_SendItemToInventory`
  (params (Item :type "/Game/Blueprints/InventoryEquipment/Struct/S_Item Structure"))
  (returns (Sended :type Boolean))
  (locals (ItemLocationRef :type "/Game/Blueprints/InventoryEquipment/Struct/S_ItemLocation Structure") (ItemArrayRef :type "Array of /Game/Blueprints/InventoryEquipment/Struct/S_Item Structure"))
  (`self.CLI_AddItemToInventory` (`local.Item`))
  (bind _output_get (set `local.ItemArrayRef` (`.Array_3_54825DA340DDAE3ADDAE89ABB7425895` (break `/Game/Blueprints/InventoryEquipment/Struct/S_ItemArray` (`BlueprintMapLibrary.Map_Find` (`self.EquipmentMap`) (`.ItemType_35_B85020CC4326255BF9CA7986369ED08C` (break `/Game/Blueprints/InventoryEquipment/Struct/S_Item` (`local.Item`))))))))
  (`KismetArrayLibrary.Array_Remove` _output_get (`.Index_5_8D07E8A340549BCF8C93F5A33213EC03` (break `/Game/Blueprints/InventoryEquipment/Struct/S_ItemLocation` (`local.ItemLocationRef`))))
  (`BlueprintMapLibrary.Map_Add` (`self.EquipmentMap`) (`.ItemType_35_B85020CC4326255BF9CA7986369ED08C` (break `/Game/Blueprints/InventoryEquipment/Struct/S_Item` (`local.Item`))) (make `/Game/Blueprints/InventoryEquipment/Struct/S_ItemArray` (`local.ItemArrayRef`)))
  (`self.ItemRemovedFromEquipment` (`local.Item`))
  (return true))

(fn `GetItemLocation`
  (params (ID :type Integer :default -1) (Item :type "/Game/Blueprints/InventoryEquipment/Struct/S_Item Structure"))
  (returns (Found :type Boolean) (ItemLocation :type "/Game/Blueprints/InventoryEquipment/Struct/S_ItemLocation Structure"))
  (bind (_value _returnvalue) (`BlueprintMapLibrary.Map_Find` (`self.InventoryIDs`) (`local.ID`)))
  (bind (_value_2 _returnvalue_2) (`BlueprintMapLibrary.Map_Find` (`self.InventoryIDs`) (`.ID_34_480AFE364D7F3357C84857B4B302F81E` (break `/Game/Blueprints/InventoryEquipment/Struct/S_Item` (`local.Item`)))))
  (if (!= ID -1)
    (return _returnvalue _value)
    (else
      (return _returnvalue_2 _value_2))))

(fn `SER_AddItemToEquipment`
  (params (Item :type "/Game/Blueprints/InventoryEquipment/Struct/S_Item Structure"))
  (returns (Added :type Boolean) (AddedItem :type "/Game/Blueprints/InventoryEquipment/Struct/S_Item Structure"))
  (locals (ItemRef :type "/Game/Blueprints/InventoryEquipment/Struct/S_Item Structure") (ItemTypeRef :type "/Game/Blueprints/InventoryEquipment/Enum/E_ItemType Enum") (ItemArrayRef :type "Array of /Game/Blueprints/InventoryEquipment/Struct/S_Item Structure") (ItemAddedIndex :type Integer) (AttachedMeshRef :type "MeshComponent Object Reference") (AttachedSocketRef :type Name :default "None") (CreatedItem :type "/Game/Blueprints/InventoryEquipment/Item/BP_ItemBase Object Reference"))
  (bind _itemref (`local.ItemRef`))
  (bind _output_get (set `local.ItemRef` Item))
  (bind _output_get_2 (set `local.ItemTypeRef` (`.ItemType_35_B85020CC4326255BF9CA7986369ED08C` (break `/Game/Blueprints/InventoryEquipment/Struct/S_Item` _output_get))))
  (bind _isthere (`self.SER_IsThereEmptySlotInEquipment` _output_get_2))
  (if _isthere
    (if (`KismetSystemLibrary.IsValidClass` (`.ItemClass_50_F3F201CE44180E709F56B981F423850B` (break `/Game/Blueprints/InventoryEquipment/Struct/S_Item` (`local.ItemRef`))))
      (bind (_mesh _socket _sockettransform) (`/Game/Blueprints/Player/BP_InGamePlayerController.GetSocket` (`self.InGamePlayerController`) (`.SocketType_53_442ADEA842922E9A87254983E4B56DD4` (break `/Game/Blueprints/InventoryEquipment/Struct/S_Item` (`local.ItemRef`)))))
      (set `local.AttachedMeshRef` _mesh)
      (set `local.AttachedSocketRef` _socket)
      (bind _returnvalue (`|SpawnActorFromClass` (`.ItemClass_50_F3F201CE44180E709F56B981F423850B` (break `/Game/Blueprints/InventoryEquipment/Struct/S_Item` (`local.ItemRef`))) _sockettransform "AlwaysSpawn" "OverrideRootScale" null (`local.ItemRef`) null))
      (bind _output_get_3 (set `local.CreatedItem` _returnvalue))
      (`Actor.K2_AttachToComponent` _output_get_3 (`local.AttachedMeshRef`) (`local.AttachedSocketRef`) "SnapToTarget" "SnapToTarget" "KeepWorld" true)
      (setmembers `/Game/Blueprints/InventoryEquipment/Struct/S_Item` :`StructRef` (`local.ItemRef`) :`ItemInstance` (`local.CreatedItem`)))
    (bind _output_get_4 (set `local.ItemArrayRef` (`.Array_3_54825DA340DDAE3ADDAE89ABB7425895` (break `/Game/Blueprints/InventoryEquipment/Struct/S_ItemArray` (`BlueprintMapLibrary.Map_Find` (`self.EquipmentMap`) (`local.ItemTypeRef`))))))
    (bind _returnvalue_2 (`KismetArrayLibrary.Array_Add` _output_get_4 (`local.ItemRef`)))
    (set `local.ItemAddedIndex` _returnvalue_2)
    (`BlueprintMapLibrary.Map_Add` (`self.EquipmentMap`) (`local.ItemTypeRef`) (make `/Game/Blueprints/InventoryEquipment/Struct/S_ItemArray` (`local.ItemArrayRef`)))
    (`KismetArrayLibrary.Array_Clear` (`local.ItemArrayRef`))
    (`BlueprintMapLibrary.Map_Add` (`self.InventoryIDs`) (`.ID_34_480AFE364D7F3357C84857B4B302F81E` (break `/Game/Blueprints/InventoryEquipment/Struct/S_Item` (`local.ItemRef`))) (make `/Game/Blueprints/InventoryEquipment/Struct/S_ItemLocation` "NewEnumerator1" (`local.ItemTypeRef`) (`local.ItemAddedIndex`)))
    (`self.ItemAddedToEquipment` _itemref)
    (return true _itemref)
    (else
      (return false))))

(fn `SER_AddItemToInventory`
  (params (Item :type "/Game/Blueprints/InventoryEquipment/Struct/S_Item Structure"))
  (returns (Added :type Boolean) (AddedItem :type "/Game/Blueprints/InventoryEquipment/Struct/S_Item Structure"))
  (locals (ItemRef :type "/Game/Blueprints/InventoryEquipment/Struct/S_Item Structure") (ItemArrayRef :type "Array of /Game/Blueprints/InventoryEquipment/Struct/S_Item Structure") (ItemAddedIndex :type Integer :default 0) (ItemTypeRef :type "/Game/Blueprints/InventoryEquipment/Enum/E_ItemType Enum"))
  (bind _itemref (`local.ItemRef`))
  (bind ((`ID_34_480AFE364D7F3357C84857B4B302F81E` _id) (`ItemType_35_B85020CC4326255BF9CA7986369ED08C` _itemtype)) (break `/Game/Blueprints/InventoryEquipment/Struct/S_Item` (`local.ItemRef`)))
  (bind _output_get (set `local.ItemRef` Item))
  (set `local.ItemTypeRef` (`.ItemType_35_B85020CC4326255BF9CA7986369ED08C` (break `/Game/Blueprints/InventoryEquipment/Struct/S_Item` _output_get)))
  (if (== (`.ID_34_480AFE364D7F3357C84857B4B302F81E` (break `/Game/Blueprints/InventoryEquipment/Struct/S_Item` (`local.ItemRef`))) -1)
    (setmembers `/Game/Blueprints/InventoryEquipment/Struct/S_Item` :`StructRef` (`local.ItemRef`) :`ID` (`self.SER_CreateNewID`))
    (else
      (bind (_found _itemlocation) (`self.GetItemLocation` -1 (`local.ItemRef`)))
      (if _found
        (switch `/Game/Blueprints/InventoryEquipment/Enum/E_ItemLocation` (`.ItemLocation_8_4E329D35476CDDB8E131009E226BCE64` (break `/Game/Blueprints/InventoryEquipment/Struct/S_ItemLocation` _itemlocation))
          (:`NewEnumerator1`
            _))
        (else
          (return false)))))
  (bind _output_get_2 (set `local.ItemArrayRef` (`.Array_3_54825DA340DDAE3ADDAE89ABB7425895` (break `/Game/Blueprints/InventoryEquipment/Struct/S_ItemArray` (`BlueprintMapLibrary.Map_Find` (`self.InventoryMap`) (`.ItemType_35_B85020CC4326255BF9CA7986369ED08C` (break `/Game/Blueprints/InventoryEquipment/Struct/S_Item` (`local.ItemRef`))))))))
  (bind _returnvalue (`KismetArrayLibrary.Array_Add` _output_get_2 (`local.ItemRef`)))
  (set `local.ItemAddedIndex` _returnvalue)
  (`BlueprintMapLibrary.Map_Add` (`self.InventoryMap`) (`local.ItemTypeRef`) (make `/Game/Blueprints/InventoryEquipment/Struct/S_ItemArray` (`local.ItemArrayRef`)))
  (`KismetArrayLibrary.Array_Clear` (`local.ItemArrayRef`))
  (`BlueprintMapLibrary.Map_Add` (`self.InventoryIDs`) _id (make `/Game/Blueprints/InventoryEquipment/Struct/S_ItemLocation` "NewEnumerator0" _itemtype (`local.ItemAddedIndex`)))
  (`self.ItemAddedToInventory` _itemref)
  (return true _itemref))

(fn `SER_CreateNewID`
  (returns (NewID :type Integer))
  (bind _keys (`BlueprintMapLibrary.Map_Keys` (`self.InventoryIDs`)))
  (return (+ (`.MaxValue` (`KismetMathLibrary.MaxOfIntArray` _keys)) 1)))

(fn `SER_IsThereEmptySlotInEquipment`
  (params (ItemType :type "/Game/Blueprints/InventoryEquipment/Enum/E_ItemType Enum" :default "NewEnumerator0"))
  (returns (IsThere :type Boolean))
  (return (< (`KismetArrayLibrary.Array_Length` (`.Array_3_54825DA340DDAE3ADDAE89ABB7425895` (break `/Game/Blueprints/InventoryEquipment/Struct/S_ItemArray` (`BlueprintMapLibrary.Map_Find` (`self.EquipmentMap`) ItemType)))) (`BlueprintMapLibrary.Map_Find` (`self.EquipmentSlotsSizes`) ItemType))))

(fn `SER_SendItemToEquipment`
  (params (Item :type "/Game/Blueprints/InventoryEquipment/Struct/S_Item Structure"))
  (returns (Sended :type Boolean) (AddedItem :type "/Game/Blueprints/InventoryEquipment/Struct/S_Item Structure"))
  (locals (ItemArrayRef :type "Array of /Game/Blueprints/InventoryEquipment/Struct/S_Item Structure") (ItemLocationRef :type "/Game/Blueprints/InventoryEquipment/Struct/S_ItemLocation Structure"))
  (bind _item (`local.Item`))
  (bind (_itemlocation _itemtype _index) (break `/Game/Blueprints/InventoryEquipment/Struct/S_ItemLocation` (`BlueprintMapLibrary.Map_Find` (`self.InventoryIDs`) (`.ID_34_480AFE364D7F3357C84857B4B302F81E` (break `/Game/Blueprints/InventoryEquipment/Struct/S_Item` (`local.Item`))))))
  (bind (_found _itemlocation_2) (`self.GetItemLocation` -1 Item))
  (if _found
    (switch `/Game/Blueprints/InventoryEquipment/Enum/E_ItemLocation` (`.ItemLocation_8_4E329D35476CDDB8E131009E226BCE64` (break `/Game/Blueprints/InventoryEquipment/Struct/S_ItemLocation` _itemlocation_2))
      (:`NewEnumerator0`
        (bind _added (`self.SER_AddItemToEquipment` (`local.Item`)))
        (if _added
          (bind _output_get (set `local.ItemArrayRef` (`.Array_3_54825DA340DDAE3ADDAE89ABB7425895` (break `/Game/Blueprints/InventoryEquipment/Struct/S_ItemArray` (`BlueprintMapLibrary.Map_Find` (`self.InventoryMap`) _itemtype)))))
          (`KismetArrayLibrary.Array_Remove` _output_get _index)
          (`BlueprintMapLibrary.Map_Add` (`self.InventoryMap`) (`.ItemType_35_B85020CC4326255BF9CA7986369ED08C` (break `/Game/Blueprints/InventoryEquipment/Struct/S_Item` (`local.Item`))) (make `/Game/Blueprints/InventoryEquipment/Struct/S_ItemArray` (`local.ItemArrayRef`)))
          (`self.ItemRemovedFromInventory` _item)
          (return true _item)
          (else
            (return false))))
      (:`NewEnumerator1`
        (return false)))
    (else
      (return false))))

(fn `SER_SendItemToInventory`
  (params (Item :type "/Game/Blueprints/InventoryEquipment/Struct/S_Item Structure"))
  (returns (Sended :type Boolean) (AddedItem :type "/Game/Blueprints/InventoryEquipment/Struct/S_Item Structure"))
  (locals (ItemLocationRef :type "/Game/Blueprints/InventoryEquipment/Struct/S_ItemLocation Structure") (ItemArrayRef :type "Array of /Game/Blueprints/InventoryEquipment/Struct/S_Item Structure"))
  (bind _item (`local.Item`))
  (bind (_found _itemlocation) (`self.GetItemLocation` -1 Item))
  (bind _output_get (set `local.ItemLocationRef` _itemlocation))
  (switch `/Game/Blueprints/InventoryEquipment/Enum/E_ItemLocation` (`.ItemLocation_8_4E329D35476CDDB8E131009E226BCE64` (break `/Game/Blueprints/InventoryEquipment/Struct/S_ItemLocation` _output_get))
    (:`NewEnumerator0`
      (return false))
    (:`NewEnumerator1`
      (bind _added (`self.SER_AddItemToInventory` (`local.Item`)))
      (if _added
        (bind _output_get_2 (set `local.ItemArrayRef` (`.Array_3_54825DA340DDAE3ADDAE89ABB7425895` (break `/Game/Blueprints/InventoryEquipment/Struct/S_ItemArray` (`BlueprintMapLibrary.Map_Find` (`self.EquipmentMap`) (`.ItemType_35_B85020CC4326255BF9CA7986369ED08C` (break `/Game/Blueprints/InventoryEquipment/Struct/S_Item` (`local.Item`))))))))
        (`KismetArrayLibrary.Array_Remove` _output_get_2 (`.Index_5_8D07E8A340549BCF8C93F5A33213EC03` (break `/Game/Blueprints/InventoryEquipment/Struct/S_ItemLocation` (`local.ItemLocationRef`))))
        (`BlueprintMapLibrary.Map_Add` (`self.EquipmentMap`) (`.ItemType_35_B85020CC4326255BF9CA7986369ED08C` (break `/Game/Blueprints/InventoryEquipment/Struct/S_Item` (`local.Item`))) (make `/Game/Blueprints/InventoryEquipment/Struct/S_ItemArray` (`local.ItemArrayRef`)))
        (`self.ItemRemovedFromEquipment` _item)
        (return true _item)
        (else
          (return false))))))