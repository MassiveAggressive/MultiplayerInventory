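; Player unit Blueprint that moves on fixed world axes and rotates to face the cursor's hit location.
; Each tick, the locally controlled unit computes a look-at yaw, applies it locally and also passes it to the S_TurnToCursor event, which sets the same rotation.
; MoveForward and MoveRight feed movement input along world X and Y.
; Logic to spawn and attach BP_MultipleWeapon at WeaponSpawnPoint is present but disconnected.
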(event `self.ReceiveBeginPlay`
  (`parent.ReceiveBeginPlay`))

(event `S_TurnToCursor`
  (params (Z :type "Float (double-precision)"))
  (`self.K2_SetActorRotation` (`KismetMathLibrary.MakeRotator` 0.0 0.0 Z)))

(event `self.ReceiveTick`
  (params (DeltaSeconds :type "Float (single-precision)"))
  (bind (_returnvalue_roll _returnvalue_pitch _returnvalue_yaw) (`KismetMathLibrary.BreakRotator` (`KismetMathLibrary.FindLookAtRotation` (`self.K2_GetActorLocation`) (`/Game/Blueprints/GeneralFunctions.GetHitLocation`))))
  (if (`self.IsLocallyControlled`)
    (`self.S_TurnToCursor` _returnvalue_yaw)
    (`self.K2_SetActorRotation` (`KismetMathLibrary.MakeRotator` 0.0 0.0 _returnvalue_yaw))))

(event `InputAxis|MoveForward`
  (params (AxisValue :type "Float (single-precision)"))
  (`self.AddMovementInput` (1.0 0.0 0.0) AxisValue))

(event `InputAxis|MoveRight`
  (params (AxisValue :type "Float (single-precision)"))
  (`self.AddMovementInput` (0.0 1.0 0.0) AxisValue))

(fn `UserConstructionScript`
  (`parent.UserConstructionScript`))