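; Player controller for the main menu that shows the menu widget and handles quitting and LAN multiplayer sessions.
; On BeginPlay it creates W_MainMenu, passes itself in and adds it to the viewport.
; Creating a game starts a two-slot LAN session and opens DevMap as a listen server.
; Searching passes the found session to the widget to build game rows, and JoinGame joins a given search result.
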(event `self.ReceiveBeginPlay`
  (bind _returnvalue (`|CreateWidget` "/Game/Blueprints/GameMode/Widget/MainMenu/W_MainMenu.W_MainMenu_C" self self))
  (bind _output_get (set `self.W_MainMenu` _returnvalue))
  (`UserWidget.AddToViewport` _output_get 0))

(event `QuitGame`
  (`KismetSystemLibrary.QuitGame` self "Quit"))

(event `CreateGame`
  (`CreateSessionCallbackProxy.CreateSession` self 2 true
    (:`OnSuccess`
      (`KismetSystemLibrary.PrintString` "CreateGame")
      (`GameplayStatics.OpenLevel` "DevMap" true "listen"))))

(event `FindGame`
  (bind _results (`FindSessionsCallbackProxy.FindSessions` self 1 true)
    (:`OnSuccess`
      (`KismetSystemLibrary.PrintString` "Found")
      (`/Game/Blueprints/GameMode/Widget/MainMenu/W_MainMenu.CreateGamesRows` (`self.W_MainMenu`) _results))
    (:`OnFailure`
      (`KismetSystemLibrary.PrintString` "Failure"))))

(event `JoinGame`
  (params (Game :type "BlueprintSessionResult Structure (by ref)"))
  (`JoinSessionCallbackProxy.JoinSession` self Game))

(fn `UserConstructionScript`
  (`parent.UserConstructionScript`))