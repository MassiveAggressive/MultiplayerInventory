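; BP_InGamePlayerController is the in-game player controller, providing socket lookup on the controlled pawn's mesh.
; GetSocket gets the pawn's mesh through a GetMeshMessage call, then queries it by socket type, returning mesh, socket and transform.
; The event graph holds only disconnected debug logic that would print stat amounts from a nested map.
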(fn `GetSocket`
  (params (SocketType :type "/Game/Blueprints/Unit/SocketsEnum/E_SocketType Enum" :default "NewEnumerator0"))
  (returns (Mesh :type "MeshComponent Object Reference") (Socket :type Name) (SocketTransform :type "Transform Structure"))
  (bind _mesh (message `/Game/Blueprints/Unit/Interface/BPI_Unit.GetMesh` (`self.K2_GetPawn`)))
  (bind (_socket _sockettransform) (message `/Game/Blueprints/Unit/Interface/BPI_Unit.GetSocket` _mesh (`local.SocketType`)))
  (return _mesh _socket _sockettransform))

(fn `UserConstructionScript`
  (`parent.UserConstructionScript`))