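; BP_InGameGameMode is the in-game game mode that picks a spawn point for each player by index.
; ChoosePlayerStart ignores the passed controller and requests the start matching the current player count minus one.
; GetPlayerStart lazily fills a PlayerStarts map from all BP_PlayerStartWithIndex actors, keyed by their PlayerIndex, then serves lookups from that cache.
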(fn `ChoosePlayerStart`
  (params (Player :type "Controller Object Reference"))
  (returns (ReturnValue :type "Actor Object Reference"))
  (bind _returnvalue (`self.GetNumPlayers`))
  (bind _playerstart (`self.GetPlayerStart` (- _returnvalue 1)))
  (return _playerstart))

(fn `GetPlayerStart`
  (params (PlayerIndex :type Integer))
  (returns (PlayerStart :type "/Game/Blueprints/Player/BP_PlayerStartWithIndex Object Reference"))
  (if (> (`BlueprintMapLibrary.Map_Length` (`self.PlayerStarts`)) 0)
    (return (`BlueprintMapLibrary.Map_Find` (`self.PlayerStarts`) (`local.PlayerIndex`)))
    (else
      (bind _outactors (`GameplayStatics.GetAllActorsOfClass` "/Game/Blueprints/Player/BP_PlayerStartWithIndex.BP_PlayerStartWithIndex_C"))
      (for _array_element _outactors
        (`BlueprintMapLibrary.Map_Add` (`self.PlayerStarts`) (`/Game/Blueprints/Player/BP_PlayerStartWithIndex.PlayerIndex` _array_element) _array_element))
      (return (`BlueprintMapLibrary.Map_Find` (`self.PlayerStarts`) (`local.PlayerIndex`))))))

(fn `UserConstructionScript`
  (`parent.UserConstructionScript`))